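; BP_item is a pickup actor for a valve, with a configurable mesh applied in the construction script.
; On BeginPlay it creates a pickup prompt widget, which shows while the player character overlaps its trigger and hides on exit.
; Its PickUp event sets HasValve on the first PlaceValveBP found in the level, prints a debug message and destroys the item.
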(event OnComponentBeginOverlap(Trigger)
  (params (OverlappedComponent :type Primitive%20Component%20Object%20Reference) (OtherActor :type Actor%20Object%20Reference) (OtherComp :type Primitive%20Component%20Object%20Reference) (OtherBodyIndex :type Integer) (bFromSweep :type Boolean) (SweepResult :type Hit%20Result%20Structure%20%28by%20ref%29))
  (if (== OtherActor (Game|GetPlayerCharacter 0))
    (UserInterface|Viewport|AddtoViewport (Variables|Default|GetPickup%20Prompt) 0)))

(event OnComponentEndOverlap(Trigger)
  (params (OverlappedComponent :type Primitive%20Component%20Object%20Reference) (OtherActor :type Actor%20Object%20Reference) (OtherComp :type Primitive%20Component%20Object%20Reference) (OtherBodyIndex :type Integer))
  (if (== OtherActor (Game|GetPlayerCharacter 0))
    (Widget|RemovefromParent (Variables|Default|GetPickup%20Prompt))))

(event EventBeginPlay
  (bind _returnvalue (UserInterface|CreateWidget "/Game/Mechanics/Pick_Up/Prompt_Pickup.Prompt_Pickup_C"))
  (Variables|Default|SetPickup%20Prompt _returnvalue))

(event Collision|EventActorBeginOverlap
  (params (OtherActor :type Actor%20Object%20Reference)))

(event EventTick
  (params (DeltaSeconds :type Float%20%28single-precision%29)))

(event EventPickUp
  (bind _returnvalue (Actor|GetActorOfClass "/Game/Mechanics/Pick_Up/PlaceValveBP.PlaceValveBP_C"))
  (Variables|/Game/Mechanics/Pick_Up/PlaceValveBP.PlaceValveBP_C|SetHasValve? _returnvalue true)
  (Development|PrintString "Valve")
  (Actor|DestroyActor))

(fn ConstructionScript
  (Components|StaticMesh|SetStaticMesh (Variables|Default|GetItemModel) (Variables|Default|GetItemModelToPlace)))