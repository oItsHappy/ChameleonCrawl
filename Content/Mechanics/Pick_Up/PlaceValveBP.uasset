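; Valve placement spot that mounts a carried valve and triggers the draining of the Pond.
; When its Box is overlapped and HasValve is set, it clears all widgets, shows the valve mesh and starts rotating it.
; It then polls with a retriggerable delay until the player overlaps the Pond's StartDrain, marks the valve placed, slowly lowers the Pond's Cube and calls ValveOverlapAllow on ValveActorComp.
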(event OnComponentBeginOverlap(Box)
  (params (OverlappedComponent :type Primitive%20Component%20Object%20Reference) (OtherActor :type Actor%20Object%20Reference) (OtherComp :type Primitive%20Component%20Object%20Reference) (OtherBodyIndex :type Integer) (bFromSweep :type Boolean) (SweepResult :type Hit%20Result%20Structure%20%28by%20ref%29))
  (bind _valvemesh (Variables|Default|GetValveMesh))
  (if (Variables|Default|GetHasValve?)
    (Viewport|RemoveAllWidgets)
    (Rendering|SetVisibility (Variables|Default|GetValveMesh) true false)
    (Components|MoveComponentTo _valvemesh (Variables|/Script/Engine.SceneComponent|GetRelativeLocation _valvemesh) "180.000000,0.000000,-90.000000" false false 2.0 false)
    (bind _returnvalue (Actor|GetActorOfClass "/Game/Mechanics/Pick_Up/Pond.Pond_C"))
    (if (Collision|IsOverlappingActor (Variables|/Game/Mechanics/Pick_Up/Pond.Pond_C|GetStartDrain _returnvalue) (Game|Player|GetPlayerPawn 0) :!class /Script/Engine.PrimitiveComponent) :!label _label
      (Variables|Default|SetValve%20Placed true)
      (Components|MoveComponentTo (Variables|/Game/Mechanics/Pick_Up/Pond.Pond_C|GetCube _returnvalue) "0.000000,0.000000,-900.000000" "0, 0, 0" false true 1e+01 false)
      (Utilities|FlowControl|Delay 1.0)
      (Default|ValveOverlapAllow (Variables|Default|GetValveActorComp))
      (else
        (Utilities|FlowControl|RetriggerableDelay 0.2)
        (goto _label)))))

(event EventBeginPlay)

(event Collision|EventActorBeginOverlap
  (params (OtherActor :type Actor%20Object%20Reference)))

(event EventTick
  (params (DeltaSeconds :type Float%20%28single-precision%29)))

(fn ConstructionScript)