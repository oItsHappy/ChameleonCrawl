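; NPC Blueprint that handles talk and pickup interactions by putting dialogue and inventory widgets on screen.
; PickUp adds the inventory widget and sets PickedUpItem, which switches Talk to an item-grabbed dialogue that removes itself after a delay.
; Otherwise Talk opens the NPC dialogue, guarded by UIOn against duplicates until the DialogueTriggerZone end overlap removes it.
; TESTDIALOGUE_1 is empty, and the debug prints are unconnected.
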(event OnComponentEndOverlap(DialogueTriggerZone)
  (params (OverlappedComponent :type Primitive%20Component%20Object%20Reference) (OtherActor :type Actor%20Object%20Reference) (OtherComp :type Primitive%20Component%20Object%20Reference) (OtherBodyIndex :type Integer))
  (Widget|RemovefromParent (Variables|Default|GetDialogueWidg))
  (Variables|Default|SetUIOn? false))

(event Custom|TESTDIALOGUE_1)

(event EventPickUp
  ;[1 1 1] InteractionEvents
  (bind _returnvalue (UserInterface|CreateWidget "/Game/UI/InventoryWidgetBP.InventoryWidgetBP_C"))
  (bind _output_get (Variables|Default|SetInventoryBPWidg _returnvalue))
  (UserInterface|Viewport|AddtoViewport _output_get 0)
  (Variables|Default|SetPickedUpItem true))

(event EventTalk
  ;[1 1 1] InteractionEvents
  (if (Variables|Default|GetPickedUpItem)
    (bind _returnvalue (UserInterface|CreateWidget "/Game/UI/ItemGrabbedDialogue.ItemGrabbedDialogue_C"))
    (bind _output_get (Variables|Default|SetGrabbedItemWidg _returnvalue))
    (UserInterface|Viewport|AddtoViewport _output_get 0)
    (Utilities|FlowControl|Delay 6.0)
    (Widget|RemovefromParent (Variables|Default|GetGrabbedItemWidg))
    (elif (not (Variables|Default|GetUIOn?))
      (Variables|Default|SetUIOn? true)
      (bind _returnvalue_2 (UserInterface|CreateWidget "/Game/UI/NPCDialogue.NPCDialogue_C"))
      (bind _output_get_2 (Variables|Default|SetDialogueWidg _returnvalue_2))
      (UserInterface|Viewport|AddtoViewport _output_get_2 0))))

(fn ConstructionScript)