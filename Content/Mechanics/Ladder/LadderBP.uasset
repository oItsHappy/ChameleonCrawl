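; LadderBP is a two-piece collectible ladder that becomes climbable once the player has picked up both pieces and reaches the build spot.
; Overlapping BoxOne or BoxTwo hides that piece, sets its flag and shows a rung widget; collecting both assigns ComponentTags to InvisibleLadder.
; Overlapping Box with both flags set removes the widgets, reveals the hidden Ladder, hides Ladder1 and calls ClimbFireEvent on CanClimb.
; Overlaps are not filtered by actor.
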(event OnComponentBeginOverlap(Box)
  (params (OverlappedComponent :type Primitive%20Component%20Object%20Reference) (OtherActor :type Actor%20Object%20Reference) (OtherComp :type Primitive%20Component%20Object%20Reference) (OtherBodyIndex :type Integer) (bFromSweep :type Boolean) (SweepResult :type Hit%20Result%20Structure%20%28by%20ref%29))
  (bind _ladder (Variables|Default|GetLadder))
  (if (Variables|Default|GetOneGrabbed)
    (if (Variables|Default|GetTwoGrabbed)
      (Widget|RemovefromParent (Variables|Default|GetRung2))
      (Widget|RemovefromParent (Variables|Default|GetRung1))
      (Rendering|SetVisibility _ladder true true)
      (Rendering|SetVisibility (Variables|Default|GetLadder1) false false)
      (Development|PrintString (Utilities|GetDisplayName _ladder))
      (Default|ClimbFireEvent (Variables|Default|GetCanClimb)))))

(event OnComponentBeginOverlap(BoxOne)
  (params (OverlappedComponent :type Primitive%20Component%20Object%20Reference) (OtherActor :type Actor%20Object%20Reference) (OtherComp :type Primitive%20Component%20Object%20Reference) (OtherBodyIndex :type Integer) (bFromSweep :type Boolean) (SweepResult :type Hit%20Result%20Structure%20%28by%20ref%29))
  (if (not (Variables|Default|GetOneGrabbed))
    (Variables|Default|SetOneGrabbed true)
    (Rendering|SetVisibility (Variables|Default|GetLadderPieceOne) false false)
    (UserInterface|Viewport|AddtoViewport (Variables|Default|GetRung1) 0)
    (if (Variables|Default|GetTwoGrabbed)
      (Variables|/Script/Engine.ActorComponent|SetComponentTags (Variables|Default|GetInvisibleLadder) (Variables|Default|GetComponent%20Tags)))))

(event OnComponentBeginOverlap(BoxTwo)
  (params (OverlappedComponent :type Primitive%20Component%20Object%20Reference) (OtherActor :type Actor%20Object%20Reference) (OtherComp :type Primitive%20Component%20Object%20Reference) (OtherBodyIndex :type Integer) (bFromSweep :type Boolean) (SweepResult :type Hit%20Result%20Structure%20%28by%20ref%29))
  (if (not (Variables|Default|GetTwoGrabbed))
    (Variables|Default|SetTwoGrabbed true)
    (Rendering|SetVisibility (Variables|Default|GetLadderPieceTwo) false false)
    (UserInterface|Viewport|AddtoViewport (Variables|Default|GetRung2) 0)
    (if (Variables|Default|GetOneGrabbed)
      (Variables|/Script/Engine.ActorComponent|SetComponentTags (Variables|Default|GetInvisibleLadder) (Variables|Default|GetComponent%20Tags)))))

(event EventBeginPlay
  (Rendering|SetVisibility (Variables|Default|GetLadder) false false))

(event Collision|EventActorBeginOverlap
  (params (OtherActor :type Actor%20Object%20Reference)))

(event EventTick
  (params (DeltaSeconds :type Float%20%28single-precision%29)))

(fn ConstructionScript)